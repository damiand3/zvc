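; Master_TestActorBP is a test actor that exercises a manager Blueprint and an integer array slicing function.
; On BeginPlay it casts ManagerReference to Master_ManagerBP, prints its status, caches it and calls SliceIntArray on a literal array without using the result.
; Tick calls PrintStatus on the cached manager every frame, with no validity check.
; A second SliceIntArray call with an out-of-range end is left unconnected.
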(event EventBeginPlay
  (bind _asmaster_manager_bp (Utilities|Casting|CastToMaster_ManagerBP (Variables|Default|GetManagerReference)))
  (Default|PrintStatus _asmaster_manager_bp)
  (Variables|Default|SetManagerRefBP _asmaster_manager_bp)
  (Class|MasterTestActor|SliceIntArray (Utilities|Array|MakeArray 1 2 3 4 5 6 7) 0 6))

(event Collision|EventActorBeginOverlap
  (params (OtherActor :type Actor%20Object%20Reference)))

(event EventTick
  (params (DeltaSeconds :type Float%20%28single-precision%29))
  (Default|PrintStatus (Variables|Default|GetManagerRefBP)))

(fn ConstructionScript)